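; BP_Cube is an actor whose static mesh bobs up and down continuously.
; BeginPlay records the mesh's starting world height.
; Each Tick accumulates elapsed time and offsets Z from that height by a degree-based sine wave scaled by Speed and Height, keeping X, Y, rotation and scale unchanged.
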(event `self.ReceiveBeginPlay`
  (bind (_returnvalue_x _returnvalue_y _returnvalue_z) (`KismetMathLibrary.BreakVector` (`SceneComponent.K2_GetComponentLocation` (`self.StaticMeshComponent`))))
  (set `self.StartHeight` _returnvalue_z))

(event `self.ReceiveTick`
  (params (DeltaSeconds :type "Float (single-precision)"))
  (bind _returnvalue (`SceneComponent.K2_GetComponentToWorld` (`self.StaticMeshComponent`)))
  (set `self.Time` (+ DeltaSeconds (`self.Time`)))
  (`SceneComponent.K2_SetWorldTransform` (`self.StaticMeshComponent`) (`KismetMathLibrary.MakeTransform` (`KismetMathLibrary.MakeVector` (.x (.location _returnvalue)) (.y (.location _returnvalue)) (+ (* (`KismetMathLibrary.DegSin` (* (`self.Time`) (`self.Speed`))) (`self.Height`)) (`self.StartHeight`))) (.rotation _returnvalue) (.scale _returnvalue)) false false))

(fn `UserConstructionScript`)